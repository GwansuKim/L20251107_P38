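; Player-controlled P38 aircraft pawn that flies forward constantly and fires missiles.
; Tick adds full movement input along the actor's forward vector, so steering comes purely from rotation.
; Pitch and Roll axes apply local rotation scaled by frame time and AxisSpeed, with no yaw input.
; Pressing Fire spawns BP_Missile at the Arrow component's world transform, with the plane as owner and instigator.
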(event EventTick
  (params (DeltaSeconds :type Float%20%28single-precision%29))
  (Utilities|FlowControl|Sequence
    (:then_0
      (Pawn|Input|AddMovementInput (Transformation|GetActorForwardVector) 1.0 false))))

(event Input|ActionEvents|InputActionFire
  (params (Key :type Key%20Structure :default "None"))
  (bind _self self)
  (:Pressed
    (Game|SpawnActorfromClass "/Game/Blueprint/P38/Misssile/BP_Missile.BP_Missile_C" (Transformation|GetWorldTransform (Variables|Default|GetArrow)) "Undefined" "MultiplyWithRoot" _self _self)))

(event Input|AxisEvents|InputAxisPitch
  (params (AxisValue :type Float%20%28single-precision%29))
  (Transformation|AddActorLocalRotation (Math|Rotator|MakeRotator 0.0 (* AxisValue (Utilities|Time|GetWorldDeltaSeconds) (Variables|Default|GetAxisSpeed)) 0.0) false false))

(event Input|AxisEvents|InputAxisRoll
  (params (AxisValue :type Float%20%28single-precision%29))
  (Transformation|AddActorLocalRotation (Math|Rotator|MakeRotator (* AxisValue (Utilities|Time|GetWorldDeltaSeconds) (Variables|Default|GetAxisSpeed)) 0.0 0.0) false false))

(fn ConstructionScript)