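; BP_Missile is a short-lived missile actor that destroys actors tagged Target when it overlaps them.
; BeginPlay sets a three-second lifespan.
; On a hit it destroys the target, then spawns a sound and a pooled emitter at the missile's location.
; The closing cast to BP_GM leads nowhere and the self-destroy node is unconnected, so the missile survives hits until its lifespan expires.
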(event EventBeginPlay
  (Actor|SetLifeSpan 3.0))

(event Collision|EventActorBeginOverlap
  (params (OtherActor :type Actor%20Object%20Reference))
  (if (Actor|ActorHasTag OtherActor "Target")
    (Actor|DestroyActor OtherActor)
    (Audio|SpawnSoundatLocation 0 (Transformation|GetActorLocation) "0, 0, 0" 1.0 1.0 0.0 0 0)
    (Effects|SpawnEmitteratLocation 0 (Transformation|GetActorLocation) "0, 0, 0" "1.000000,1.000000,1.000000" true "AutoRelease")
    (Utilities|Casting|CastToBP_GM (Game|GetGameMode))))

(fn ConstructionScript)